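; Weapon item Blueprint that lets the player equip it and fire projectiles.
; Activating or disabling it sets the player character's weapon-in-hand state, with a brief equipped flag on activation and aiming cleared on disable.
; Using it while aiming spawns the Projectile class at the mesh's BulletSpawnLocation socket and decrements ammo, which starts full at BeginPlay.
; An empty magazine only prints a reload message, with no reload logic in this graph.
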(event `self.ReceiveBeginPlay`
  (`parent.ReceiveBeginPlay`)
  (set `self.currentAmmo` (`self.maxAmmo`)))

(event `/Game/Items/IUseable.Disable Item`
  (bind _asplayer_character_bp (cast `/Game/Characters/PlayerCharacter_BP` (`GameplayStatics.GetPlayerPawn` 0))
    (:`then`
      (set `/Game/Characters/PlayerCharacter_BP.hasWeaponInHand` false _asplayer_character_bp)
      (set `/Game/Characters/PlayerCharacter_BP.isAiming` false _asplayer_character_bp))
    (:`CastFailed`
      (`KismetSystemLibrary.PrintString` "No player"))))

(event `/Game/Items/IUseable.ActivateItem`
  (bind _asplayer_character_bp (cast `/Game/Characters/PlayerCharacter_BP` (`GameplayStatics.GetPlayerPawn` 0))
    (:`then`
      (set `/Game/Characters/PlayerCharacter_BP.hasWeaponInHand` true _asplayer_character_bp)
      (set `/Game/Characters/PlayerCharacter_BP.hasBeenEquipped` true _asplayer_character_bp)
      (`KismetSystemLibrary.Delay` 0.7)
      (set `/Game/Characters/PlayerCharacter_BP.hasBeenEquipped` false _asplayer_character_bp))
    (:`CastFailed`
      (`KismetSystemLibrary.PrintString` "No player"))))

(event `/Game/Items/IUseable.UseItem`
  (bind _weaponmesh (`self.WeaponMesh`))
  ;[1 1 1] Spawn bullet and fire.
  (bind _asplayer_character_bp (cast `/Game/Characters/PlayerCharacter_BP` (`GameplayStatics.GetPlayerPawn` 0)))
  (if (`/Game/Characters/PlayerCharacter_BP.isAiming` _asplayer_character_bp)
    (if (> (`self.currentAmmo`) 0)
      (`|SpawnActorFromClass` "/Game/Items/Weapons/Bullets/Projectile.Projectile_C" (`KismetMathLibrary.MakeTransform` (`SceneComponent.GetSocketLocation` _weaponmesh "BulletSpawnLocation") (`SceneComponent.GetSocketRotation` _weaponmesh "BulletSpawnLocation")) "Undefined" "OverrideRootScale" null null)
      (bind _output_get (set `self.currentAmmo` (- (`self.currentAmmo`) 1)))
      (`KismetSystemLibrary.PrintString` (`KismetStringLibrary.Conv_IntToString` _output_get))
      (else
        (`KismetSystemLibrary.PrintString` "reload!")))))

(fn `UserConstructionScript`
  (`parent.UserConstructionScript`))